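; TiendaBP is a shop actor that lets the player open a store UI while standing inside its collision volume.
; Player overlap toggles IsInRange and adds or removes a message widget.
; Tick polls the Q key to open TiendaUI with UI-only input and a visible cursor.
; Tick also sets its PointOfInterestComponent's EsVisible flag by comparing the shop's Piso (floor) to the player's floor in the GlobalInstances game instance.
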(event OnComponentBeginOverlap(Collision)
  (params (OverlappedComponent :type Primitive%20Component%20Object%20Reference) (OtherActor :type Actor%20Object%20Reference) (OtherComp :type Primitive%20Component%20Object%20Reference) (OtherBodyIndex :type Integer) (bFromSweep :type Boolean) (SweepResult :type Hit%20Result%20Structure%20%28by%20ref%29))
  ;[1 1 1] EnterCollision
  (Utilities|FlowControl|Sequence
    (:then_0
      (if (== OtherActor (Game|GetPlayerCharacter 0))
        (Variables|Default|SetIsInRange true)
        (bind _returnvalue (UserInterface|CreateWidget "/Game/BPs/Tienda/TiendaMsgUI.TiendaMsgUI_C" (Game|GetPlayerController 0)))
        (bind _output_get (Variables|Default|Setmessage _returnvalue))
        (UserInterface|Viewport|AddtoViewport _output_get 0)))))

(event OnComponentEndOverlap(Collision)
  (params (OverlappedComponent :type Primitive%20Component%20Object%20Reference) (OtherActor :type Actor%20Object%20Reference) (OtherComp :type Primitive%20Component%20Object%20Reference) (OtherBodyIndex :type Integer))
  ;[1 1 1] ExitCollision
  (if (== OtherActor (Game|GetPlayerCharacter 0))
    (Variables|Default|SetIsInRange false)
    (Development|PrintString "Exit")
    (Variables|Default|SetTiendaUI 0)
    (Widget|RemovefromParent (Variables|Default|Getmessage))))

(event EventTick
  (params (DeltaSeconds :type Float%20%28single-precision%29))
  (bind _returnvalue (Game|GetPlayerController 0))
  ;[1 1 1] Mostrar Icono
  (Utilities|FlowControl|Sequence
    (:then_0
      ;[1 1 1] Abir tienda
      (Utilities|IsValid (Variables|Default|GetTiendaUI)
        (:Is%20Not%20Valid
          (if (and (== (Class|PlayerController|GetInputAnalogKeyState (Game|GetPlayerController 0) "Q") 1.0) (Variables|Default|GetIsInRange))
            (bind _returnvalue_2 (UserInterface|CreateWidget "/Game/BPs/Tienda/TiendaUI.TiendaUI_C" (Game|GetPlayerController 0)))
            (UserInterface|Viewport|AddtoViewport _returnvalue_2 0)
            (bind _output_get (Variables|Default|SetTiendaUI _returnvalue_2))
            (Input|SetInputModeUIOnly _returnvalue _output_get "DoNotLock")
            (Variables|/Script/Engine.PlayerController|SetbShowMouseCursor _returnvalue true)))))
    (:then_1
      (bind _asglobal_instances (Utilities|Casting|CastToGlobalInstances (Game|GetGameInstance)))
      (Variables|/Game/ThirdPersonBP/Minimap/PointOfInterest_Component.PointOfInterest_Component_C|SetesVisible (Variables|Default|GetPointOfInterest_Component) (== (Variables|/Game/GlobalInstances.GlobalInstances_C|GetPisoJugador _asglobal_instances) (Variables|Default|GetPiso))))))

(fn ConstructionScript)