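; BP_Desperfecto is a breakable fixture that randomly breaks, costing money, and pays a reward when repaired.
; Tick drives the random break delay, camera-facing warning text and point-of-interest visibility.
; Overlap tracks player range and shows a repair widget while broken.
; Holding E in range with the required tool advances progress per frame, resetting on release; breaks and repairs update money and broken count in GlobalInstances.
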(event OnComponentBeginOverlap(Collision)
  (params (OverlappedComponent :type Primitive%20Component%20Object%20Reference) (OtherActor :type Actor%20Object%20Reference) (OtherComp :type Primitive%20Component%20Object%20Reference) (OtherBodyIndex :type Integer) (bFromSweep :type Boolean) (SweepResult :type Hit%20Result%20Structure%20%28by%20ref%29))
  ;[1 1 1] EnterCollision
  (if (== OtherActor (Game|GetPlayerCharacter 0))
    (Variables|Default|SetIs%20In%20Range true)
    (Development|PrintString "Enter")
    (if (Variables|Default|GetBroken)
      (bind _returnvalue (UserInterface|CreateWidget "/Game/BPs/Desperfecto/UI_Desperfecto.UI_Desperfecto_C" (Game|GetPlayerController 0)))
      (UserInterface|Viewport|AddtoViewport _returnvalue 0)
      (Variables|Default|SetUI_BarraReparar _returnvalue)
      (Variables|/Game/BPs/Desperfecto/UI_Desperfecto.UI_Desperfecto_C|SetDesperfecto _returnvalue self))))

(event OnComponentEndOverlap(Collision)
  (params (OverlappedComponent :type Primitive%20Component%20Object%20Reference) (OtherActor :type Actor%20Object%20Reference) (OtherComp :type Primitive%20Component%20Object%20Reference) (OtherBodyIndex :type Integer))
  ;[1 1 1] ExitCollision
  (if (== OtherActor (Game|GetPlayerCharacter 0))
    (Variables|Default|SetIs%20In%20Range false)
    (Development|PrintString "Exit")
    (if (Variables|Default|GetBroken)
      (Widget|RemovefromParent (Variables|Default|GetUI_BarraReparar)))))

(event EventBeginPlay
  (bind _mesh (Variables|Default|GetMesh))
  (Utilities|FlowControl|Sequence
    (:then_0
      (Variables|/Game/ThirdPersonBP/Minimap/PointOfInterest_Component.PointOfInterest_Component_C|SetPisoasd (Variables|Default|GetPointOfInterest_Component) (Variables|Default|GetPiso)))
    (:then_1
      ;[1 1 1] Posem de comentari el nom del Desperfecte
      (Rendering|Components|TextRender|SetText (Variables|Default|GetTextAvis) (Utilities|Text|ToText(String) (Utilities|String|Append "Reparar " (Utilities|String|ToString(Name) (Variables|Default|GetName)) " amb " (Utilities|String|ToString(Name) (Variables|Default|GetHerramientaNecesaria))))))
    (:then_2
      ;[1 1 1] Si hay mesh adjudicado, cambialo
      (if (Utilities|IsValid _mesh)
        (Components|StaticMesh|SetStaticMesh (Variables|Default|GetCube) _mesh)))))

(event EventTick
  (params (DeltaSeconds :type Float%20%28single-precision%29))
  ;[1 1 1] Mostrar/Ocultar icono roto
  (Utilities|FlowControl|Sequence
    (:then_0
      ;[1 1 1] Destruir Aleatoriamente
      (CallFunction|TextLooktoCamera)
      (if (Variables|Default|GetBroken)
        ;[1 1 1] Reparar
        (if (Math|Boolean|ANDBoolean (== (Class|PlayerController|GetInputAnalogKeyState (Game|GetPlayerController 0) "E") 1.0) (Variables|Default|GetBroken) (Variables|Default|GetIs%20In%20Range))
          (bind _asglobal_instances (Utilities|Casting|CastToGlobalInstances (Game|GetGameInstance)))
          (if (Utilities|Name|Equal(Name) (Variables|/Game/GlobalInstances.GlobalInstances_C|GetHerramienta _asglobal_instances) (Variables|Default|GetHerramientaNecesaria))
            (Development|PrintString "Puedes reparar con esto")
            (bind _asglobal_instances_2 (Utilities|Casting|CastToGlobalInstances (Game|GetGameInstance)))
            (if (== 1.0 (Math|Conversions|ToFloat(Integer) (Utilities|Array|Get(acopy) (Variables|/Game/GlobalInstances.GlobalInstances_C|GetEfectividadHerramienta _asglobal_instances_2))))
              (CallFunction|Reparar))
            (else
              (Development|PrintString "No puedes reparar con esto")))
          (else
            (Variables|Default|SetActualRepair 0.0)))
        (else
          (Utilities|FlowControl|Delay (Math|Random|RandomFloatinRange (Variables|Default|GetDestructionMinTime) (Variables|Default|GetDestructionMaxTime)))
          (Variables|Default|SetBroken true)
          (Variables|Default|SetActualRepair 0.0)
          (Development|PrintString "Destruido!")
          (Rendering|SetVisibility (Variables|Default|GetTextAvis) true false)
          (bind _asglobal_instances_3 (Utilities|Casting|CastToGlobalInstances (Game|GetGameInstance)))
          (Variables|/Game/GlobalInstances.GlobalInstances_C|SetDinero _asglobal_instances_3 (- (Variables|/Game/GlobalInstances.GlobalInstances_C|GetDinero _asglobal_instances_3) 50))
          (bind _asglobal_instances_4 (Utilities|Casting|CastToGlobalInstances (Game|GetGameInstance)))
          (bind _result (Math|Integer|IncrementInt (Variables|/Game/GlobalInstances.GlobalInstances_C|GetnumeroRotos _asglobal_instances_4))
            (:%20%20
              (bind _output_get (Variables|/Game/GlobalInstances.GlobalInstances_C|SetnumeroRotos _asglobal_instances_4 _result))
              (Development|PrintString (Utilities|String|ToString(Integer) _output_get))
              (if (Variables|Default|GetIs%20In%20Range)
                (bind _returnvalue (UserInterface|CreateWidget "/Game/BPs/Desperfecto/UI_Desperfecto.UI_Desperfecto_C" (Game|GetPlayerController 0)))
                (UserInterface|Viewport|AddtoViewport _returnvalue 0)
                (Variables|Default|SetUI_BarraReparar _returnvalue)
                (Variables|/Game/BPs/Desperfecto/UI_Desperfecto.UI_Desperfecto_C|SetDesperfecto _returnvalue self)))))))
    (:then_1
      (Variables|/Game/ThirdPersonBP/Minimap/PointOfInterest_Component.PointOfInterest_Component_C|SetesVisible (Variables|Default|GetPointOfInterest_Component) (Variables|Default|GetBroken)))))

(fn ConstructionScript)

(fn Reparar
  ;[1 1 1] Se ejecuta cada frame que el jugador esta reparando
  (if (> 1.0 (Variables|Default|GetActualRepair))
    (Variables|Default|SetActualRepair (+ (Variables|Default|GetActualRepair) (Variables|Default|GetRepairRate)))
    (else
      (Variables|Default|SetBroken false)
      (Widget|RemovefromParent (Variables|Default|GetUI_BarraReparar))
      (Rendering|SetVisibility (Variables|Default|GetTextAvis) false false)
      (bind _asglobal_instances (Utilities|Casting|CastToGlobalInstances (Game|GetGameInstance)))
      (Variables|/Game/GlobalInstances.GlobalInstances_C|SetDinero _asglobal_instances (+ (Variables|/Game/GlobalInstances.GlobalInstances_C|GetDinero _asglobal_instances) (Variables|Default|GetRecompensa)))
      (bind _asglobal_instances_2 (Utilities|Casting|CastToGlobalInstances (Game|GetGameInstance)))
      (bind _result (Math|Integer|DecrementInt (Variables|/Game/GlobalInstances.GlobalInstances_C|GetnumeroRotos _asglobal_instances_2))
        (:%20%20
          (Variables|/Game/GlobalInstances.GlobalInstances_C|SetnumeroRotos _asglobal_instances_2 _result))))))

(fn TextLooktoCamera
  (bind _textavis (Variables|Default|GetTextAvis))
  (Transformation|SetWorldRotation _textavis (.Rotation (Math|Transform|BreakTransform (Transformation|GetActorTransform (Game|GetPlayerCameraManager 0)))) false false)
  (Transformation|AddLocalRotation _textavis "0,-180.000000, 0" false false))